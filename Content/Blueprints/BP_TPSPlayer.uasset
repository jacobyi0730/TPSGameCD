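; Third-person shooter player Blueprint whose only live logic plays a camera shake through the player camera manager when Fire is pressed.
; The other input, Tick and BeginPlay events are empty.
; Disconnected, never-executed graphs hold movement, look, jump, crouch, sprint-style speed changes, dive roll, FOV zoom, and firing via montage, sound, bullet spawn or physics-pushing line trace.
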(event `self.ReceiveBeginPlay`)

(event `InputAxis|Look Up / Down Mouse` :overrideparent false
  (params (AxisValue :type "Float (single-precision)")))

(event `InputAxis|Turn Right / Left Mouse` :overrideparent false
  (params (AxisValue :type "Float (single-precision)")))

(event `InputAction|Jump` :overrideparent false
  (params (Key :type "Key Structure")))

(event `InputAction|Fire` :overrideparent false
  (params (Key :type "Key Structure"))
  (:`Pressed`
    (`PlayerCameraManager.StartCameraShake` :`self` (`GameplayStatics.GetPlayerCameraManager` 0) :`ShakeClass` "/Game/Blueprints/BP_FireCameraShake.BP_FireCameraShake_C")))

(event `InputAction|Zoom` :overrideparent false
  (params (Key :type "Key Structure")))

(event `InputAction|ActionRun` :overrideparent false
  (params (Key :type "Key Structure")))

(event `self.ReceiveTick`
  (params (DeltaSeconds :type "Float (single-precision)")))

(event `InputAction|ActionCrouch` :overrideparent false
  (params (Key :type "Key Structure")))

(event `InputAction|DiveRoll` :overrideparent false
  (params (Key :type "Key Structure")))

(fn `UserConstructionScript`)