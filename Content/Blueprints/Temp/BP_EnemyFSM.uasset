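; Enemy AI state machine that runs on Tick inside a component owned by BP_Enemy, cycling through IDLE, MOVE and ATTACK.
; IDLE caches the player character as target and the owner as the pawn to drive.
; MOVE steers straight at the target with AddMovementInput until within AttackDist.
; ATTACK waits on a Delay, prints a placeholder attack message, then returns to MOVE if the target's 2D distance is out of range.
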(event `self.ReceiveTick`
  (params (DeltaSeconds :type "Float (single-precision)"))
  (bind _returnvalue (`GameplayStatics.GetPlayerCharacter` 0))
  (bind _returnvalue_2 (- (`Actor.K2_GetActorLocation` (`self.target`)) (`Actor.K2_GetActorLocation` (`self.me`))))
  (switch `/Game/Blueprints/Temp/BP_EEnemyState` (`self.state`)
    (:`NewEnumerator0`
      ;[1 1 1] Idle : 주인공을 찾아서 목적지로 기억하고싶다. 만약 목적지가 있다면 이동상태로 전이하고싶다.
      (`/Engine/EditorBlueprintResources/StandardMacros.IsValid` _returnvalue
        (:`Is Valid`
          (set `self.target` _returnvalue)
          (bind _asbp_enemy (cast `/Game/Blueprints/BP_Enemy` (`self.GetOwner`)))
          (set `self.me` _asbp_enemy)
          (set `self.state` "NewEnumerator1"))))
    (:`NewEnumerator1`
      ;[1 1 1] Move : 목적지를 향해 이동하고싶다. 만약 목적지와의 거리가 3M이내라면 공격상태로 전이하고싶다.
      (`Pawn.AddMovementInput` (`self.me`) _returnvalue_2 1.0 false)
      (if (< (`KismetMathLibrary.VSize` _returnvalue_2) (`self.attackDist`))
        (set `self.state` "NewEnumerator2")))
    (:`NewEnumerator2`
      ;[1 1 1] Attack : 2초 대기했다가 공격을 하고 싶다. 만약 공격을 하려고할때 목적지와의 거리가 3M를 초과한다면 이동상태로 전이하고싶다.
      (`KismetSystemLibrary.Delay` 2.0)
      (`KismetSystemLibrary.PrintString` "Attack" true true (struct :`G` 0.66 :`B` 1.0 :`A` 1.0) 10.0)
      (if (>= (`KismetMathLibrary.Vector_Distance2D` (`Actor.K2_GetActorLocation` (`self.target`)) (`Actor.K2_GetActorLocation` (`self.me`))) (`self.attackDist`))
        (set `self.state` "NewEnumerator1")))))